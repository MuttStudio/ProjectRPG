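; Player controller for ProjectRPG that relays item-handling modifier keys to the player pawn.
; Either Shift key toggles split-items mode and either Ctrl key toggles single-item mode, sent on press and release as messages to player pawn 0.
; Releasing the left mouse button sets CurrentDrag back to its first enum value.
; The construction script casts and caches the HUD as BP_ProjectRPGHUD.
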(event Input|KeyboardEvents|RightShift
  (bind _returnvalue (Game|Player|GetPlayerPawn 0))
  (:Pressed
    (Class|BPInterface|SplitItems(Message) _returnvalue true))
  (:Released
    (Class|BPInterface|SplitItems(Message) _returnvalue false)))

(event Input|KeyboardEvents|RightCtrl
  (bind _returnvalue (Game|Player|GetPlayerPawn 0))
  (:Pressed
    (Class|BPInterface|SingleItem(Message) _returnvalue true))
  (:Released
    (Class|BPInterface|SingleItem(Message) _returnvalue false)))

(event Input|KeyboardEvents|LeftCtrl
  (bind _returnvalue (Game|Player|GetPlayerPawn 0))
  (:Pressed
    (Class|BPInterface|SingleItem(Message) _returnvalue true))
  (:Released
    (Class|BPInterface|SingleItem(Message) _returnvalue false)))

(event Input|KeyboardEvents|LeftShift
  (bind _returnvalue (Game|Player|GetPlayerPawn 0))
  (:Pressed
    (Class|BPInterface|SplitItems(Message) _returnvalue true))
  (:Released
    (Class|BPInterface|SplitItems(Message) _returnvalue false)))

(event Input|MouseEvents|LeftMouseButton
  (:Released
    (Variables|Default|SetCurrentDrag "NewEnumerator0")))

(fn ConstructionScript
  (bind _asbp_projectrpghud_c (Utilities|Casting|CastToBP_ProjectRPGHUD (HUD|GetHUD)))
  (Variables|Default|SetHUD _asbp_projectrpghud_c))