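; Player character Blueprint for ProjectRPG that handles held items and inventory/item-bar slot operations, and forwards quest-offer and item-hover messages to the HUD.
; SwapItems and RemoveItem parse slot names by prefix (I for inventory, B for bar) plus index, with split and single flags setting moved stack size.
; EquipItem attaches items to a hand socket, StoweItem destroys the current one, and temporary BeginPlay test code spawns an axe weapon on authority.
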(event EventDisplayItemHover
  (params (NewItem :type Project%20RPG%20Item%20Object%20Reference))
  (Class|BPCharacterEvents|CharacterViewItem(Message) (HUD|GetHUD (Game|GetPlayerController 0)) NewItem))

(event EventDisplayQuestOffer
  (Class|BPCharacterEvents|DisplayQuestOffer(Message) (HUD|GetHUD (Game|GetPlayerController 0)) (Variables|Default|GetQuestOffer)))

(event EventSplitItems
  (params (IsSplitting :type Boolean))
  ;[1 1 1] I think we can delete these
  (Variables|Default|SetIsSplitting IsSplitting))

(event EventBeginPlay
  ;[1 1 1] Testing Code - DELETE ME
  (Networking|SwitchHasAuthority
    (:Authority
      (bind _returnvalue (Game|SpawnActorfromClass "/Game/Meshes/Items/BP_Axe1.BP_Axe1_C" (Math|Transform|MakeTransform "0, 0,25.000000") false 0))
      (Variables|Default|SetAxe _returnvalue)
      (Class|Actor|AttachRootComponentto (Variables|Default|GetAxe) (Variables|Character|GetMesh) "hand_socket_l" "KeepRelativeOffset")
      (Variables|/Script/ProjectRPG.ProjectRPGItem|SetControllingPawn (Variables|Default|GetAxe) (Game|Player|GetPlayerPawn 0))
      (Variables|Default|SetCurrentWeapon (Variables|Default|GetAxe))
      (Variables|/Script/ProjectRPG.ProjectRPGItem|SetItemOwner (Variables|Default|GetAxe) self))))

(event EventSingleItem
  (params (IsSingle :type Boolean))
  ;[1 1 1] I think we can delete these
  (Variables|Default|SetIsSingle IsSingle))

(fn ConstructionScript)

(fn EquipItem
  (params (Item :type Project%20RPG%20Item%20Object%20Reference))
  (Class|Actor|AttachRootComponentto Item (Variables|Character|GetMesh) "RightItemSocket" "SnapToTarget")
  (Variables|Default|SetCurrentItem Item))

(fn StoweItem
  (Actor|DestroyActor (Variables|Default|GetCurrentItem)))

(fn SwapItems
  (params (To :type Name) (From :type Name))
  (bind _returnvalue (Utilities|String|ToString(Name) To))
  (bind _returnvalue_2 (Utilities|String|ToString(Name) From))
  (bind _returnvalue_3 (Utilities|String|GetSubstring _returnvalue 0))
  (bind _returnvalue_4 (Utilities|String|GetSubstring _returnvalue_2 0))
  (bind _returnvalue_5 (Utilities|String|Len _returnvalue_2))
  (bind _returnvalue_6 (Utilities|String|Len _returnvalue))
  (bind _returnvalue_7 (Utilities|Enum|Equal(Enum) _returnvalue_4 "I"))
  (bind _returnvalue_8 (- _returnvalue_5 1))
  (bind _returnvalue_9 (- _returnvalue_6 1))
  (bind _returnvalue_10 (Utilities|Enum|Equal(Enum) _returnvalue_3 "B"))
  (bind _returnvalue_11 (Utilities|String|GetSubstring _returnvalue_2 1 _returnvalue_8))
  (bind _returnvalue_12 (Utilities|String|GetSubstring _returnvalue 1 _returnvalue_9))
  (bind _returnvalue_13 (Math|Conversions|ToInteger(Byte) _returnvalue_11))
  (bind _returnvalue_14 (Math|Conversions|ToInteger(Byte) _returnvalue_12))
  (if (and _returnvalue_7 (Utilities|Enum|Equal(Enum) _returnvalue_3 "I"))
    (if (Variables|Default|GetIsSplitting)
      (bind _asprojectrpgcharacter (Utilities|Casting|CastToProjectRPGCharacter (Game|Player|GetPlayerPawn 0)))
      (bind _returnvalue_15 (Class|ProjectRPGCharacter|GetCurrentInventory _asprojectrpgcharacter))
      (LocalVariables|SetStackSize_0 (/ (Variables|/Script/ProjectRPG.ProjectRPGItem|GetStackSize (Utilities|Array|Get(acopy) _returnvalue_15 _returnvalue_13)) 2))
      (elif (Variables|Default|GetIsSingle)
        (LocalVariables|SetStackSize_0 1)
        (else
          (LocalVariables|SetStackSize_0 0))))
    (Class|ProjectRPGCharacter|MoveItem _returnvalue_13 _returnvalue_14 (LocalVariables|GetStackSize_0))
    (elif (and _returnvalue_10 _returnvalue_7)
      (Class|ProjectRPGCharacter|AddItemtoItemBar _returnvalue_13 _returnvalue_14)
      (elif (and _returnvalue_10 (Utilities|Enum|Equal(Enum) _returnvalue_4 "B"))
        (Class|ProjectRPGCharacter|MoveItemonBar _returnvalue_14 _returnvalue_13)))))

(fn RemoveItem
  (params (Remove :type Name) (HUD :type BP%20Project%20RPGHUD%20Object%20Reference))
  (bind _returnvalue (Utilities|String|ToString(Name) Remove))
  (bind _returnvalue_2 (Utilities|String|Len _returnvalue))
  (bind _returnvalue_3 (- _returnvalue_2 1))
  (bind _returnvalue_4 (Utilities|String|GetSubstring _returnvalue 1 _returnvalue_3))
  (bind _returnvalue_5 (Math|Conversions|ToInteger(Byte) _returnvalue_4))
  (switch string (Utilities|String|GetSubstring _returnvalue 0)
    (:B
      (Class|ProjectRPGCharacter|RemoveItemBarItem _returnvalue_5))
    (:I
      (Class|ProjectRPGCharacter|RemoveItemfromInventory _returnvalue_5))))