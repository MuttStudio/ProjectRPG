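; Character Blueprint that handles equipping held items and rearranging inventory and item bar slots.
; EquipItem snaps an item to the mesh's right-hand socket as CurrentItem, and StoweItem destroys that actor.
; SwapItems parses slot names made of an "I" or "B" prefix plus an index to move items within the inventory, from inventory to bar, or along the bar.
; Bar-to-inventory moves have no branch.
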(fn ConstructionScript)

(fn EquipItem
  (params (Item :type Project%20RPG%20Item%20Object%20Reference))
  (Class|Actor|AttachRootComponentto Item (Variables|Character|GetMesh) "RightItemSocket" "SnapToTarget")
  (Variables|Default|SetCurrentItem Item))

(fn StoweItem
  (Actor|DestroyActor (Variables|Default|GetCurrentItem)))

(fn SwapItems
  (params (To :type Name) (From :type Name))
  (bind _returnvalue (Utilities|String|ToString(Name) To))
  (bind _returnvalue_2 (Utilities|String|ToString(Name) From))
  (bind _returnvalue_3 (Utilities|String|GetSubstring _returnvalue 0))
  (bind _returnvalue_4 (Utilities|String|GetSubstring _returnvalue_2 0))
  (bind _returnvalue_5 (Utilities|String|Len _returnvalue_2))
  (bind _returnvalue_6 (Utilities|String|Len _returnvalue))
  (bind _returnvalue_7 (Utilities|Enum|Equal(Enum) _returnvalue_4 "I"))
  (bind _returnvalue_8 (- _returnvalue_5 1))
  (bind _returnvalue_9 (- _returnvalue_6 1))
  (bind _returnvalue_10 (Utilities|Enum|Equal(Enum) _returnvalue_3 "B"))
  (bind _returnvalue_11 (Utilities|String|GetSubstring _returnvalue_2 1 _returnvalue_8))
  (bind _returnvalue_12 (Utilities|String|GetSubstring _returnvalue 1 _returnvalue_9))
  (bind _returnvalue_13 (Math|Conversions|ToInteger(Byte) _returnvalue_11))
  (bind _returnvalue_14 (Math|Conversions|ToInteger(Byte) _returnvalue_12))
  (if (and _returnvalue_7 (Utilities|Enum|Equal(Enum) _returnvalue_3 "I"))
    (Class|ProjectRPGCharacter|MoveItem _returnvalue_13 _returnvalue_14)
    (elif (and _returnvalue_10 _returnvalue_7)
      (Class|ProjectRPGCharacter|AddItemtoItemBar _returnvalue_13 _returnvalue_14)
      (elif (and _returnvalue_10 (Utilities|Enum|Equal(Enum) _returnvalue_4 "B"))
        (Class|ProjectRPGCharacter|MoveItemonBar _returnvalue_14 _returnvalue_13)))))